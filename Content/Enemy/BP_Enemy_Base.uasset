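; Base enemy character Blueprint that provides rifle equipping, attacking, patrol route access and movement speed control.
; EquipRifle spawns a BP_Rifle, snaps it to the mesh's hand socket and flags it as equipped.
; Attack plays a firing montage and calls OnAttackEnd whether it completes or is interrupted.
; SetMovementSpeed maps an idle, walking or sprinting state to max walk speed, and GetPatrolRoute returns the stored route.
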(event Custom|Equip%20Rifle
  (bind _returnvalue (Game|SpawnActorfromClass "/Game/Enemy/Enemy_Weapon/BP_Rifle.BP_Rifle_C" (Transformation|GetActorTransform) "Undefined" "MultiplyWithRoot" 0 0))
  (Transformation|AttachComponentToComponent _returnvalue (Variables|Character|GetMesh) "RightHandRifle" "SnapToTarget" "SnapToTarget" "SnapToTarget" true)
  (Variables|Default|SetIsRifleEquiped true))

(event Custom|Attack
  (Animation|Montage|PlayMontage (Variables|Character|GetMesh) "/Game/Enemy/Enemy_Animations/Firing_Rifle_Montage.Firing_Rifle_Montage"
    (:OnCompleted
      _)
    (:OnInterrupted
      _))
  (Default|CallOnAttackEnd))

(event EventBeginPlay)

(fn ConstructionScript)

(fn GetPatrolRoute
  (return (Variables|AI|GetPatrolRoute)))

(fn SetMovementSpeed
  (params (Speed :type E_MovementSpeed%20Enum :default "NewEnumerator0"))
  (bind _output_get (Variables|/Script/Engine.CharacterMovementComponent|SetMaxWalkSpeed (Variables|Character|GetCharacterMovement) (Utilities|Select :Index Speed :NewEnumerator0 0.0 :NewEnumerator1 1e+02 :NewEnumerator2 5e+02)))
  (return _output_get))