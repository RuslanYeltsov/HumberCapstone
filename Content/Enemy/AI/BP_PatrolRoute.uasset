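; BP_PatrolRoute is an enemy AI patrol path actor that defines waypoints along a PatrolRoute spline.
; IncrementPatrolRoute advances PatrolIndex by PatrolDir and flips the direction at the first and last spline points, producing a back-and-forth patrol.
; GetSplinePointAsWorldPos returns the current point's world location.
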(event Custom|Increment%20Patrol%20Route
  (bind _output_get (Variables|Default|SetPatrolIndex (+ (Variables|Default|GetPatrolIndex) (Variables|Default|GetPatrolDir))))
  (if (== _output_get (- (Spline|GetNumberOfSplinePoints (Variables|Default|GetPatrolRoute)) 1))
    (Variables|Default|SetPatrolDir -1)
    (elif (== (Variables|Default|GetPatrolIndex) 0)
      (Variables|Default|SetPatrolDir 1))))

(fn ConstructionScript)

(fn GetSplinePointasWorldPos
  (return (Spline|GetLocationatSplinePoint (Variables|Default|GetPatrolRoute) (Variables|Default|GetPatrolIndex) "World")))