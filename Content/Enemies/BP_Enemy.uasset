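; Enemy Blueprint that walks a looping patrol route through placed BP_PatrolPoint actors.
; From BeginPlay, it uses AIMoveTo toward each point by index, pausing briefly after each successful move before calling Patrol again, and returns to the first when the index runs out.
; AddNavPoints spawns owner-linked point actors from relative PatrolPath offsets, and the construction script rebuilds those offsets from the point actors' positions.
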(event Custom|Patrol
  (if (<= (Variables|Default|GetCurrentPatrolPoint) (Utilities|Array|Length (Variables|Default|GetPatrolPath)))
    (AI|AIMoveTo self (Transformation|GetActorLocation (Utilities|Array|Get(acopy) (Variables|Default|GetPatrolPathPoints) (Variables|Default|GetCurrentPatrolPoint))) 0 5.0 false
      (:then
        (Math|Integer|IncrementInt (Variables|Default|GetCurrentPatrolPoint)))
      (:OnSuccess
        (Utilities|FlowControl|Delay 0.5 :!label _label)
        (CallFunction|Patrol)))
    (else
      (AI|AIMoveTo self (Transformation|GetActorLocation (Utilities|Array|Get(acopy) (Variables|Default|GetPatrolPathPoints))) 0 5.0 false
        (:then
          (Variables|Default|SetCurrentPatrolPoint 1))
        (:OnSuccess
          (goto _label))))))

(event Custom|AddNavPoints
  (for _array_element (Variables|Default|GetPatrolPath)
    (bind _returnvalue (Game|SpawnActorfromClass "/Game/Enemies/BP_PatrolPoint.BP_PatrolPoint_C" (Math|Transform|MakeTransform (+ _array_element (Transformation|GetActorLocation)) "0, 0, 0" "1.000000,1.000000,1.000000") "Undefined" "MultiplyWithRoot" 0 0))
    (Variables|/Game/Enemies/BP_PatrolPoint.BP_PatrolPoint_C|SetEnemyOwner _returnvalue self)
    (Utilities|Array|Add (Variables|Default|GetPatrolPathPoints) _returnvalue)))

(event EventBeginPlay
  (if (<= (Variables|Default|GetCurrentPatrolPoint) (Utilities|Array|Length (Variables|Default|GetPatrolPath)))
    (AI|AIMoveTo self (Transformation|GetActorLocation (Utilities|Array|Get(acopy) (Variables|Default|GetPatrolPathPoints) (Variables|Default|GetCurrentPatrolPoint))) 0 5.0 false
      (:then
        (Math|Integer|IncrementInt (Variables|Default|GetCurrentPatrolPoint)))
      (:OnSuccess
        (Utilities|FlowControl|Delay 0.5 :!label _label)
        (CallFunction|Patrol)))
    (else
      (AI|AIMoveTo self (Transformation|GetActorLocation (Utilities|Array|Get(acopy) (Variables|Default|GetPatrolPathPoints))) 0 5.0 false
        (:then
          (Variables|Default|SetCurrentPatrolPoint 1))
        (:OnSuccess
          (goto _label))))))

(fn ConstructionScript
  (if (Utilities|Array|IsNotEmpty (Variables|Default|GetPatrolPathPoints))
    (Utilities|Array|Clear (Variables|Default|GetPatrolPath))
    (for _array_element (Variables|Default|GetPatrolPathPoints)
      (Utilities|Array|Add (Variables|Default|GetPatrolPath) (- (Transformation|GetActorLocation _array_element) (Transformation|GetActorLocation))))))